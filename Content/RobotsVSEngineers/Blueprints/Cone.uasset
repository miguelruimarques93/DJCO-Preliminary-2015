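; Cone is a faction headquarters actor that registers itself with the RvE game state on BeginPlay.
; Clicking it spawns a unit of the configured class at its spawn point, then gives that unit its default controller.
; Tick runs a repeating resource-generation countdown, but on expiry it only resets the timer and checks the game state, without granting resources.
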(event OnClicked(Cone)
  (params (TouchedComponent :type Primitive%20Component%20Object%20Reference))
  (bind _returnvalue (Class|RobotsVSEngineersFunctionLibrary|SpawnUnit self (Variables|Default|GetActorToSpawn) (Transformation|GetActorLocation (Variables|Default|GetSpawn%20Point))))
  (Utilities|IsValid _returnvalue
    (:Is%20Valid
      (Pawn|SpawnDefaultController _returnvalue))))

(event EventTick
  (params (DeltaSeconds :type Float%20%28single-precision%29))
  (bind _output_get (Variables|Default|SetTimeToGenerateResources (- (Variables|Default|GetTimeToGenerateResources) DeltaSeconds)))
  (if (<= _output_get 0.0)
    (Variables|Default|SetTimeToGenerateResources 1e+01)
    (Utilities|IsValid (Game|GetGameState))))

(event EventBeginPlay
  (bind _returnvalue (Game|GetGameState))
  (Utilities|IsValid _returnvalue
    (:Is%20Valid
      (bind _asrv_egame_state (Utilities|Casting|CastToRvEGameState _returnvalue))
      (Class|RvEGameState|SetFactionHeadquarter _asrv_egame_state self))))

(fn ConstructionScript)