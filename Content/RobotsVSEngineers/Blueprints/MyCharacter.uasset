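; MyCharacter is a character Blueprint that can move to a stored destination actor.
; The construction script switches the mesh to Animation Blueprint mode using TopDownAnimBlueprint.
; SetDestination stores the goal, and MoveToDestination sends the controller toward it with SimpleMoveToActor and prints a debug string.
; A Moving flag gates the move request, and none of these graphs clears it.
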(fn ConstructionScript
  (Components|Animation|SetAnimationMode "AnimationBlueprint")
  (Components|SkeletalMesh|SetAnimInstanceClass "/Game/RobotsVSEngineers/Character/TopDownAnimBlueprint.TopDownAnimBlueprint_C"))

(fn MovetoDestination
  (if (not (Variables|Default|GetMoving))
    (Variables|Default|SetMoving true)
    (AI|Navigation|SimpleMovetoActor (Pawn|GetController) (Variables|Default|GetDestination))
    (Development|PrintString "Hello")))

(fn SetDestination
  (params (NewParam :type Actor%20Object%20Reference))
  (Variables|Default|SetDestination NewParam))